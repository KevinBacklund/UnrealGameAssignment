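; BP_Base is the player's base: it takes damage from overlapping enemies, destroys them, and drives waves and win/lose state.
; BeginPlay creates the HUD, binds health death and controller resource events, and starts the first enemy wave.
; Tick accumulates time to spawn further waves through EnemyManager at randomized offset locations.
; GameOver pauses and shows win or loss when health runs out or the final wave is cleared.
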(event `UpdateResourceCounter`
  (params (CurrentResources :type "Float (single-precision)"))
  (set `TextBlock.Text` (`KismetTextLibrary.Conv_DoubleToText` CurrentResources "HalfToEven") (`/Game/BP_HUD.CurrentResources` (`self.HUD`))))

(event `self.ReceiveBeginPlay`
  (bind _enemies_to_spawn (`self.Enemies to Spawn`))
  (add `HealthComponent.OnDeath` (`self.Health`) (delegate `GameOver`))
  (bind _asmy_player_controller (cast `MyPlayerController` (`GameplayStatics.GetPlayerController` 0)))
  (add `MyPlayerController.OnResourceChanged` _asmy_player_controller (delegate `UpdateResourceCounter`))
  (bind _returnvalue (`|CreateWidget` "/Game/BP_HUD.BP_HUD_C"))
  (bind _output_get (set `self.HUD` _returnvalue))
  (`UserWidget.AddToViewport` _output_get 0)
  (`self.UpdateHealthBar`)
  (for _ (range 11)
    (`KismetArrayLibrary.Array_Add` _enemies_to_spawn "/Game/BP_Enemy.BP_Enemy_C"))
  (`EnemyManager.SpawnNextWave` (subsystem `EnemyManager`) _enemies_to_spawn (2000.0 0.0 0.0) 2.0)
  (bind _asmy_player_controller_2 (cast `MyPlayerController` (`GameplayStatics.GetPlayerController` 0)))
  (`self.UpdateResourceCounter` (`MyPlayerController.Resources` _asmy_player_controller_2)))

(event `GameOver`
  (`GameplayStatics.SetGamePaused` true)
  (bind _returnvalue (`|CreateWidget` "/Game/BP_GameOverScreen.BP_GameOverScreen_C"))
  (`UserWidget.AddToViewport` _returnvalue 0)
  (if (`HealthComponent.IsDead` (`self.Health`))
    (bind _gameovertext (`/Game/BP_GameOverScreen.GameOverText` _returnvalue))
    (set `TextBlock.Text` "You Lost" _gameovertext)
    (else
      (set `TextBlock.Text` "You Win" _gameovertext))))

(event `UpdateHealthBar`
  (bind _health (`self.Health`))
  (set `/Game/BP_HUD.HealthPercent` (/ (`HealthComponent.CurrentHealth` _health) (`HealthComponent.MaxHealth` _health)) (`self.HUD`)))

(event `self.ReceiveTick`
  (params (DeltaSeconds :type "Float (single-precision)"))
  (bind _returnvalue (subsystem `EnemyManager`))
  (bind _minspawndistance (`self.MinSpawnDistance`))
  (bind _output_get (set `self.Acc` (+ DeltaSeconds (`self.Acc`))))
  (if (> _output_get (`self.TimeToNextWave`))
    (set `self.Acc` 0.0)
    (`EnemyManager.SpawnNextWave` _returnvalue (`self.Enemies to Spawn`) (+ (`KismetMathLibrary.RandomPointInBoundingBox` (0.0 0.0 0.0) (1000.0 1000.0 0.0)) (`KismetMathLibrary.MakeVector` _minspawndistance _minspawndistance)) 0.5))
  (if (and (>= (`EnemyManager.CurrentWave` _returnvalue) (`self.NumberOfWaves`)) (`KismetArrayLibrary.Array_IsEmpty` (`EnemyManager.GetEnemies` _returnvalue)))
    (`self.GameOver`)))

(event `self.ReceiveActorBeginOverlap`
  (params (OtherActor :type "Actor Object Reference"))
  (bind _asenemy (cast `Enemy` OtherActor))
  (`HealthComponent.TakeDamage` (`self.Health`) (`Enemy.Damage` _asenemy))
  (`self.UpdateHealthBar`)
  (`self.K2_DestroyActor` _asenemy))

(fn `UserConstructionScript`)