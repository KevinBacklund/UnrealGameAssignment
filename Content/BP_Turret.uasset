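; BP_Turret is a turret actor that fires projectiles at enemies and takes damage when they reach it.
; An overlapping Enemy passes its Damage to the Health component and is destroyed.
; The Health component's death event, bound on BeginPlay, destroys the turret.
; A custom fire event spawns BP_Projectile at the turret's transform with the supplied target; this graph contains no targeting or timing logic.
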(event `self.ReceiveBeginPlay`
  (add `HealthComponent.OnDeath` (`self.Health`) (delegate `OnDeath`)))

(event `OnDeath`
  (`self.K2_DestroyActor`))

(event `self.ReceiveActorBeginOverlap`
  (params (OtherActor :type "Actor Object Reference"))
  (bind _asenemy (cast `Enemy` OtherActor))
  (`HealthComponent.TakeDamage` (`self.Health`) (`Enemy.Damage` _asenemy))
  (`self.K2_DestroyActor` _asenemy))

(event `self.FireAtTargetEnemy`
  (params (Target :type "Vector Structure"))
  (`|SpawnActorFromClass` "/Game/BP_Projectile.BP_Projectile_C" (`self.GetTransform`) "Undefined" "MultiplyWithRoot" null Target null))

(fn `UserConstructionScript`)