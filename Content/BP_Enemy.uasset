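; BP_Enemy is an enemy actor that periodically picks a turret as its target and is destroyed when it dies.
; Tick checks the Health death state each frame and accumulates delta time as a two-second retarget timer.
; Each time the timer fires, a sphere overlap around the enemy gathers nearby BP_Turret actors and passes a random one to SetTarget, without checking for an empty result.
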(event `self.ReceiveTick`
  (params (DeltaSeconds :type "Float (single-precision)"))
  (`|ExecutionSequence`
    (:`then_0`
      (if (`HealthComponent.IsDead` (`self.Health`))
        (`self.K2_DestroyActor`)))
    (:`then_1`
      (bind _output_get (set `self.Acc` (+ DeltaSeconds (`self.Acc`))))
      (if (>= _output_get 2.0)
        (set `self.Acc` 0.0)
        (bind _outactors (`KismetSystemLibrary.SphereOverlapActors` (`self.K2_GetActorLocation`) 350.0 (`|MakeArray` "ObjectTypeQuery2" :!type "EObjectTypeQuery Enum") "/Game/BP_Turret.BP_Turret_C"))
        (`self.SetTarget` (`KismetArrayLibrary.Array_Random` _outactors))))))

(fn `UserConstructionScript`)